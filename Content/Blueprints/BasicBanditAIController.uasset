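; AI controller for bandits that activate as a group and capture a strongbox at the camp center.
; While idle and alive, it rolls a frame-time-scaled random activation chance each tick, and damage also triggers activation.
; Activation uses a sphere overlap to switch on nearby BasicBandit controllers.
; Once active, it stores CampCenterWaypoint locations as its destination and accumulates capture time when close, without issuing movement itself.
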(event EventBeginPlay)

(event EventTick
  (params (DeltaSeconds :type Float%20%28single-precision%29))
  (bind _asfirst_person_character (Utilities|Casting|CastToFirstPersonCharacter (Pawn|GetControlledPawn)))
  (if (> (Variables|/Script/LD35.LD35Character|GetHealth _asfirst_person_character) 0.0)
    (if (Variables|Default|GetIsActivated)
      (bind _outactors (Actor|GetAllActorsOfClass "/Game/Blueprints/CampCenterWaypoint.CampCenterWaypoint_C"))
      (for _array_element _outactors
        (bind _output_get (Variables|Default|SetCurrentDestination (Transformation|GetActorLocation _array_element)))
        (if (< (Math|Vector|VectorLength (- _output_get (Transformation|GetActorLocation (Pawn|GetControlledPawn)))) 2e+02)
          (Variables|Default|SetStrongboxCapture (+ (Variables|Default|GetStrongboxCapture) DeltaSeconds))
          (Development|PrintString "Bandit is capturing strongbox" false)))
      (elif (<= (Math|Random|RandomFloat) (/ DeltaSeconds (Variables|Default|GetActivationOdds)))
        (Development|PrintString "Bandit activated!" false)
        (bind _outactors_2 (Class|KismetSystemLibrary|SphereOverlapActorsNEW (Transformation|GetActorLocation (Pawn|GetControlledPawn)) 1.5e+03 (Utilities|Array|MakeArray "ObjectTypeQuery3") "/Game/Blueprints/BasicBandit.BasicBandit_C"))
        (for _array_element_2 _outactors_2
          (bind _aspawn (Utilities|Casting|CastToPawn _array_element_2))
          (bind _asbasic_bandit_aicontroller (Utilities|Casting|CastToBasicBanditAIController (Pawn|GetController _aspawn)))
          (Variables|BasicBanditAIController_C|SetIsActivated _asbasic_bandit_aicontroller true)
          (Development|PrintString (Utilities|String|Append (Utilities|GetDisplayName _aspawn) " has been activated") false))))))

(event Game|Damage|EventAnyDamage
  (params (Damage :type Float%20%28single-precision%29) (DamageType :type Damage%20Type%20Object%20Reference) (InstigatedBy :type Controller%20Object%20Reference) (DamageCauser :type Actor%20Object%20Reference))
  (if (not (Variables|Default|GetIsActivated))
    (Development|PrintString "Bandit activated!" false)
    (bind _outactors (Class|KismetSystemLibrary|SphereOverlapActorsNEW (Transformation|GetActorLocation (Pawn|GetControlledPawn)) 1.5e+03 (Utilities|Array|MakeArray "ObjectTypeQuery3") "/Game/Blueprints/BasicBandit.BasicBandit_C"))
    (for _array_element _outactors
      (bind _aspawn (Utilities|Casting|CastToPawn _array_element))
      (bind _asbasic_bandit_aicontroller (Utilities|Casting|CastToBasicBanditAIController (Pawn|GetController _aspawn)))
      (Variables|BasicBanditAIController_C|SetIsActivated _asbasic_bandit_aicontroller true)
      (Development|PrintString (Utilities|String|Append (Utilities|GetDisplayName _aspawn) " has been activated") false))))

(fn ConstructionScript)