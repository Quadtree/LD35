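; AI controller for defenders that keeps its pawn wandering around the camp center.
; Each Tick, when path following reports no active move, it looks up the first CampCenterWaypoint actor in the level.
; It then moves to that waypoint's location plus a random horizontal offset within a square bounded by PatrolSize.
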(event EventBeginPlay)

(event EventTick
  (params (DeltaSeconds :type Float%20%28single-precision%29))
  (bind _patrolsize (Variables|Default|GetPatrolSize))
  (bind _returnvalue (- 0.0 _patrolsize))
  (if (== (Class|PathFollowingComponent|GetPathActionType (Variables|Default|GetPathFollowingComponent)) (Utilities|Enum|LiteralenumEPathFollowingAction "NoMove"))
    (bind _outactors (Actor|GetAllActorsOfClass "/Game/Blueprints/CampCenterWaypoint.CampCenterWaypoint_C"))
    (AI|Navigation|MovetoLocation (+ (Transformation|GetActorLocation (Utilities|Array|Get(acopy) _outactors)) (Math|Vector|MakeVector (Math|Random|RandomFloatinRange _returnvalue _patrolsize) (Math|Random|RandomFloatinRange _returnvalue _patrolsize) 0.0)) -1.0 true true false)))

(fn ConstructionScript)